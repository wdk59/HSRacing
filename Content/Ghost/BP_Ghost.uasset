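; BP_Ghost is a short-lived ghost actor that fades out and destroys itself.
; SetGhostLife uses IsRight to choose a spooky cat mesh (right) or ghost mesh (left), with dynamic M_GhostFade materials on its slots.
; A per-mesh timeline lowers the fadeOut parameter, then destroys the actor on finish.
; Tick calls a latent MoveComponentTo targeting a point above the mesh's world location, passed as a relative location.
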(event Custom|SetGhostLife
  (params (bIsRight? :type Boolean))
  (if bIsRight?
    ;[1 1 1] 오른쪽: Spooky Cat
    (Components|StaticMesh|SetStaticMesh (Variables|Default|GetSM_Ghost) "/Game/Assets/Ghosts/SpookyCat/cute_spooky_cat.cute_spooky_cat")
    (bind _returnvalue (Rendering|Material|CreateDynamicMaterialInstance (Variables|Default|GetSM_Ghost) 0 "/Game/Ghost/M_GhostFade.M_GhostFade" "None" :!class /Script/Engine.PrimitiveComponent))
    (bind _returnvalue_2 (Rendering|Material|CreateDynamicMaterialInstance (Variables|Default|GetSM_Ghost) 1 "/Game/Ghost/M_GhostFade.M_GhostFade" "None" :!class /Script/Engine.PrimitiveComponent))
    (bind _returnvalue_3 (Rendering|Material|CreateDynamicMaterialInstance (Variables|Default|GetSM_Ghost) 2 "/Game/Ghost/M_GhostFade.M_GhostFade" "None" :!class /Script/Engine.PrimitiveComponent))
    (bind _fadetime (Timeline|Fade_SpookyCat PlayFromStart)
      (:Update
        (Rendering|Material|SetScalarParameterValue _returnvalue "fadeOut" (Math|Float|Lerp 1.0 0.0 _fadetime) :!class /Script/Engine.MaterialInstanceDynamic)
        (Rendering|Material|SetScalarParameterValue _returnvalue_2 "fadeOut" (Math|Float|Lerp 1.0 0.0 _fadetime) :!class /Script/Engine.MaterialInstanceDynamic)
        (Rendering|Material|SetScalarParameterValue _returnvalue_3 "fadeOut" (Math|Float|Lerp 1.0 0.0 _fadetime) :!class /Script/Engine.MaterialInstanceDynamic))
      (:Finished
        (Actor|DestroyActor)))
    (else
      ;[1 1 1] 왼쪽: Ghost
      (Components|StaticMesh|SetStaticMesh (Variables|Default|GetSM_Ghost) "/Game/Assets/Ghosts/Ghost/rigged_animated_ghost.rigged_animated_ghost")
      (bind _returnvalue_4 (Rendering|Material|CreateDynamicMaterialInstance (Variables|Default|GetSM_Ghost) 0 "/Game/Ghost/M_GhostFade.M_GhostFade" "None" :!class /Script/Engine.PrimitiveComponent))
      (bind _fadetime_2 (Timeline|Fade_Ghost PlayFromStart)
        (:Update
          (Rendering|Material|SetScalarParameterValue _returnvalue_4 "fadeOut" (Math|Float|Lerp 1.0 0.0 _fadetime_2) :!class /Script/Engine.MaterialInstanceDynamic))
        (:Finished
          (Actor|DestroyActor))))))

(event EventBeginPlay)

(event Collision|EventActorBeginOverlap
  (params (OtherActor :type Actor%20Object%20Reference)))

(event EventTick
  (params (DeltaSeconds :type Float%20%28single-precision%29))
  (Components|MoveComponentTo 0 (+ (Transformation|GetWorldLocation (Variables|Default|GetSM_Ghost)) "0, 0,500.000000") (Transformation|GetWorldRotation (Variables|Default|GetSM_Ghost)) false false 2.0 false))

(fn ConstructionScript)