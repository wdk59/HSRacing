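; BP_Shadow is a short-lived shadow effect actor built from StaticMesh and CatBusLeg meshes that destroys itself.
; On BeginPlay it applies M_Shadow to both meshes with a random "Random" parameter, then a timeline animates the material's "Alpha" until the actor is destroyed.
; An unconnected variant does the same on a PoseableMesh that copies a skeletal mesh's pose, like an afterimage.
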(event EventBeginPlay
  (bind _staticmesh (Variables|Default|GetStaticMesh))
  (Rendering|Material|SetMaterial _staticmesh 0 "/Game/Blueprints/Material/M_Shadow.M_Shadow")
  (Rendering|Material|SetMaterial _staticmesh 1 "/Game/Blueprints/Material/M_Shadow.M_Shadow")
  (Rendering|Material|SetScalarParameterValueonMaterials (Variables|Default|GetStaticMesh) "Random" (Math|Random|RandomFloat))
  (bind _새_트랙_0 (Timeline|타임라인_1 PlayFromStart)
    (:Update
      (Rendering|Material|SetScalarParameterValueonMaterials (Variables|Default|GetStaticMesh) "Alpha" _새_트랙_0))
    (:Finished
      (Actor|DestroyActor))))

(event Collision|EventActorBeginOverlap
  (params (OtherActor :type Actor%20Object%20Reference)))

(event EventTick
  (params (DeltaSeconds :type Float%20%28single-precision%29)))

(fn ConstructionScript)