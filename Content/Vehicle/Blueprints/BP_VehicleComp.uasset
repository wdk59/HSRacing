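; Vehicle component that releases ghosts from the owning vehicle's windows when it crashes, while souls remain.
; OnCrash picks one random index across the left and right window offset arrays, treated as a single range.
; It spawns a BP_Ghost at that unrotated offset from the owner's location, with per-side rotation and scale.
; It passes a right-side flag to SetGhostLife, then decrements SoulNum.
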(event EventBeginPlay)

(event EventTick
  (params (DeltaSeconds :type Float%20%28single-precision%29)))

(fn OnCrash
  (bind _windowloc_l (Variables|Default|GetWindowLoc_L))
  (bind _returnvalue (Utilities|Array|Length _windowloc_l))
  (if (> (Variables|Default|GetSoulNum) 0)
    (bind _output_get (LocalVariables|SetLocIndex (Math|Random|RandomIntegerinRange 0 (- (+ _returnvalue (Utilities|Array|Length (Variables|Default|GetWindowLoc_R))) 1))))
    (if (< (- _returnvalue 1) _output_get)
      ;[1 1 1] 오른쪽 창문
      (bind _returnvalue_2 (Game|SpawnActorfromClass "/Game/Ghost/BP_Ghost.BP_Ghost_C" (Math|Transform|MakeTransform (+ (Utilities|Array|Get(acopy) (Variables|Default|GetWindowLoc_R) (- (LocalVariables|GetLocIndex) _returnvalue)) (Transformation|GetActorLocation (Components|GetOwner))) "0.000000,-90.000000, 0" "0.300000,0.300000,0.300000") "Undefined" 0 0))
      (Default|SetGhostLife _returnvalue_2 (< (- _returnvalue 1) _output_get))
      (else
        ;[1 1 1] 왼쪽 창문
        (bind _returnvalue_3 (Game|SpawnActorfromClass "/Game/Ghost/BP_Ghost.BP_Ghost_C" (Math|Transform|MakeTransform (+ (Utilities|Array|Get(acopy) (Variables|Default|GetWindowLoc_L) (LocalVariables|GetLocIndex)) (Transformation|GetActorLocation (Components|GetOwner))) "0.000000,0.000000, 0" "0.500000,0.500000,0.500000") "Undefined" 0 0))
        (Default|SetGhostLife _returnvalue_3 (< (- _returnvalue 1) _output_get))))
    (Math|Integer|DecrementInt (Variables|Default|GetSoulNum))))