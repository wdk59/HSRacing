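; BP_HSRasing is a racing vehicle Blueprint with a CatBus body that handles boost shadows and crash reactions.
; A looping timer spawns BP_Shadow actors at the body's transform while boosting, leaving a trail of copies behind.
; Front, back, left, right and roof hit detectors share one overlap handler that calls OnCrash on the vehicle component.
; A shock flag, cleared by a timer, blocks repeated crashes during the shock window.
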(event OnComponentBeginOverlap(HitDetector_F)
  (params (OverlappedComponent :type Primitive%20Component%20Object%20Reference) (OtherActor :type Actor%20Object%20Reference) (OtherComp :type Primitive%20Component%20Object%20Reference) (OtherBodyIndex :type Integer) (bFromSweep :type Boolean) (SweepResult :type Hit%20Result%20Structure%20%28by%20ref%29))
  (if (not (Variables|Default|GetbIsShocking?))
    (Variables|Default|SetbIsShocking? true)
    (Utilities|Time|SetTimerbyEvent (delegate Custom|EscapeCrashShock) (Variables|Default|GetCrashShockTime))
    (Default|OnCrash (Variables|Default|GetBP_VehicleComp))))

(event OnComponentBeginOverlap(HitDetector_B)
  (params (OverlappedComponent :type Primitive%20Component%20Object%20Reference) (OtherActor :type Actor%20Object%20Reference) (OtherComp :type Primitive%20Component%20Object%20Reference) (OtherBodyIndex :type Integer) (bFromSweep :type Boolean) (SweepResult :type Hit%20Result%20Structure%20%28by%20ref%29))
  (if (not (Variables|Default|GetbIsShocking?))
    (Variables|Default|SetbIsShocking? true)
    (Utilities|Time|SetTimerbyEvent (delegate Custom|EscapeCrashShock) (Variables|Default|GetCrashShockTime))
    (Default|OnCrash (Variables|Default|GetBP_VehicleComp))))

(event OnComponentBeginOverlap(HitDetector_L)
  (params (OverlappedComponent :type Primitive%20Component%20Object%20Reference) (OtherActor :type Actor%20Object%20Reference) (OtherComp :type Primitive%20Component%20Object%20Reference) (OtherBodyIndex :type Integer) (bFromSweep :type Boolean) (SweepResult :type Hit%20Result%20Structure%20%28by%20ref%29))
  (if (not (Variables|Default|GetbIsShocking?))
    (Variables|Default|SetbIsShocking? true)
    (Utilities|Time|SetTimerbyEvent (delegate Custom|EscapeCrashShock) (Variables|Default|GetCrashShockTime))
    (Default|OnCrash (Variables|Default|GetBP_VehicleComp))))

(event OnComponentBeginOverlap(HitDetector_R)
  (params (OverlappedComponent :type Primitive%20Component%20Object%20Reference) (OtherActor :type Actor%20Object%20Reference) (OtherComp :type Primitive%20Component%20Object%20Reference) (OtherBodyIndex :type Integer) (bFromSweep :type Boolean) (SweepResult :type Hit%20Result%20Structure%20%28by%20ref%29))
  (if (not (Variables|Default|GetbIsShocking?))
    (Variables|Default|SetbIsShocking? true)
    (Utilities|Time|SetTimerbyEvent (delegate Custom|EscapeCrashShock) (Variables|Default|GetCrashShockTime))
    (Default|OnCrash (Variables|Default|GetBP_VehicleComp))))

(event OnComponentBeginOverlap(HitDetector_Roof)
  (params (OverlappedComponent :type Primitive%20Component%20Object%20Reference) (OtherActor :type Actor%20Object%20Reference) (OtherComp :type Primitive%20Component%20Object%20Reference) (OtherBodyIndex :type Integer) (bFromSweep :type Boolean) (SweepResult :type Hit%20Result%20Structure%20%28by%20ref%29))
  (if (not (Variables|Default|GetbIsShocking?))
    (Variables|Default|SetbIsShocking? true)
    (Utilities|Time|SetTimerbyEvent (delegate Custom|EscapeCrashShock) (Variables|Default|GetCrashShockTime))
    (Default|OnCrash (Variables|Default|GetBP_VehicleComp))))

(event Custom|EscapeCrashShock
  (Variables|Default|SetbIsShocking? false))

(event Custom|MakeShadow
  (if (Variables|Default|GetisBoost)
    (Game|SpawnActorfromClass "/Game/Blueprints/Material/BP_Shadow.BP_Shadow_C" (Transformation|GetWorldTransform (Variables|Default|GetCatBus_Body)) "Undefined" 0 0)))

(event EventBeginPlay
  (Utilities|Time|SetTimerbyEvent (delegate Custom|MakeShadow) 0.25 true))

(event Collision|EventActorBeginOverlap
  (params (OtherActor :type Actor%20Object%20Reference)))

(event EventTick
  (params (DeltaSeconds :type Float%20%28single-precision%29)))

(fn ConstructionScript)