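; A single cat bus leg actor that rotates while its vehicle, a BP_HSRasing found as the owner's owner, is moving.
; Each Tick above a small speed threshold, it adds ShakingDir to the leg's world pitch and zeroes roll and yaw.
; ShakingDir steps toward zero only at magnitude five or more, and the running total in Cnt is never read.
; Tick also prints the owner's name as debug output.
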(event EventBeginPlay)

(event Collision|EventActorBeginOverlap
  (params (OtherActor :type Actor%20Object%20Reference)))

(event EventTick
  (params (DeltaSeconds :type Float%20%28single-precision%29))
  (bind _returnvalue (Components|GetOwner))
  (Development|PrintString (Utilities|GetObjectName _returnvalue))
  (bind _asbp_hsrasing (Utilities|Casting|CastToBP_HSRasing (Components|GetOwner _returnvalue)))
  (if (> (Math|Vector|VectorLength (Transformation|GetVelocity _asbp_hsrasing)) 2e+01)
    (Transformation|SetWorldRotation (Variables|Default|GetCatBus_OneLeg) (Math|Rotator|MakeRotator 0.0 (+ (Variables|Default|GetShakingDir) (.pitch (Transformation|GetWorldRotation (Variables|Default|GetCatBus_OneLeg)))) 0.0) false false)
    (Variables|Default|Setcnt (+ (Variables|Default|GetShakingDir) (Variables|Default|Getcnt)))
    (if (<= 5.0 (Variables|Default|GetShakingDir))
      (Variables|Default|SetShakingDir (+ (Variables|Default|GetShakingDir) -1.0))
      (elif (<= (Variables|Default|GetShakingDir) -5.0)
        (Variables|Default|SetShakingDir (+ (Variables|Default|GetShakingDir) 1.0))))))

(fn ConstructionScript)